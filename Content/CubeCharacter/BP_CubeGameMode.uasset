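; BP_CubeGameMode is the game mode for the cube character game and owns its HUD.
; On BeginPlay it constructs a BPW_CubeUI widget for player 0 and stores it as UIRef without displaying it.
; Separate events add the widget to the viewport and write time and point values into its text fields.
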(event EventBeginPlay
  (CallFunction|InitializeUI))

(event EventTick
  (params (DeltaSeconds :type Float%20%28single-precision%29)))

(event Custom|UpdateUITime
  (params (Time :type Float%20%28double-precision%29))
  ;[0.004456 0.01581 0.15 0.5] UI Time
  (Rendering|Components|TextRender|SetText (Variables|/Game/UI/BPW_CubeUI.BPW_CubeUI_C|GetTimeValue (Variables|UI|GetUIRef)) (Utilities|Text|ToText(Float) Time "HalfToEven")))

(event Custom|UpdateUIPoints
  (params (Points :type Float%20%28double-precision%29))
  ;[0.000538 0 0.15 0.5] UI Points
  (Rendering|Components|TextRender|SetText (Variables|/Game/UI/BPW_CubeUI.BPW_CubeUI_C|GetPointValue (Variables|UI|GetUIRef)) (Utilities|Text|ToText(Float) Points "HalfToEven")))

(event Custom|InitializeUI
  ;[0.01925 0.03052 0.15 0.5] Init UI
  (bind _returnvalue (Game|ConstructObjectfromClass (Game|GetPlayerController 0) "/Game/UI/BPW_CubeUI.BPW_CubeUI_C"))
  (Variables|UI|SetUIRef _returnvalue))

(event Custom|ShowUI
  ;[0.01731 0.03334 0.15 0.5] Show UI
  (UserInterface|Viewport|AddtoViewport (Variables|UI|GetUIRef) 0))

(fn ConstructionScript)