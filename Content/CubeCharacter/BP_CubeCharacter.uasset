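; BP_CubeCharacter is a player character with spring arm camera, walk, look and jump, plus a toggle that turns the player into a dead cube.
; The first MakeCube press saves velocity, hides the body, disables movement and collision, then spawns a BP_DeadCubeCharacter that inherits that velocity.
; The next press teleports the character to the PlayerStart and restores visibility, collision and walking, leaving the spawned cube behind.
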(event Input|ActionEvents|InputActionJump
  (params (Key :type Key%20Structure :default "None"))
  ;[0.15 0.02469 0.02469 0.5] Input
  (:Pressed
    (Character|Jump)))

(event Input|ActionEvents|InputActionMakeCube
  (params (Key :type Key%20Structure :default "None"))
  ;[0.1344 0.001536 0.15 0.5] Spawn Cube Mechanic
  (:Pressed
    (if (not (Variables|Default|GetbPlayerMakeCubeState))
      ;;[0.15 0.15 0.15 0.5] KIll Cube and Spawn Ghost Cube
      (CallFunction|MakeCubeandSetInvisible false)
      (|SpawnCube)
      (Variables|Default|SetbPlayerMakeCubeState true)
      (else
        ;;[0.15 0.15 0.15 0.5] Respawn Player At Start
        (bind _returnvalue (Actor|GetActorOfClass "/Script/Engine.PlayerStart"))
        (Transformation|SetActorLocationAndRotation (.location (Transformation|GetActorTransform _returnvalue)) (.rotation (Transformation|GetActorTransform _returnvalue)))
        (CallFunction|MakeCubeandSetInvisible true)
        (Variables|Default|SetbPlayerMakeCubeState false)))))

(event Input|AxisEvents|InputAxisMoveForwardBackwards
  (params (AxisValue :type Float%20%28single-precision%29))
  ;[0.15 0.05156 0.05156 0.5] Move WASD
  (Pawn|Input|AddMovementInput (Transformation|GetActorForwardVector (Pawn|GetController)) AxisValue false))

(event Input|AxisEvents|InputAxisMoveLeftRight
  (params (AxisValue :type Float%20%28single-precision%29))
  ;[0.15 0.05156 0.05156 0.5] Move WASD
  (Pawn|Input|AddMovementInput (Transformation|GetActorRightVector (Pawn|GetController)) AxisValue false))

(event Input|AxisEvents|InputAxisLookUpDown
  (params (AxisValue :type Float%20%28single-precision%29))
  ;[0.15 0.01409 0.07013 0.5] Look Mouse
  (Pawn|Input|AddControllerPitchInput AxisValue))

(event Input|AxisEvents|InputAxisLookLeftRight
  (params (AxisValue :type Float%20%28single-precision%29))
  ;[0.15 0.01409 0.07013 0.5] Look Mouse
  (Pawn|Input|AddControllerYawInput AxisValue))

(fn ConstructionScript)

(fn MakeCubeandSetInvisible
  (params (Reverse :type Boolean))
  ;[0.15 0.04516 0.06773 0.5] Kill Cube
  (Utilities|FlowControl|Sequence
    (:then_0
      (Variables|Default|SetVelocityOnMakeCube (Transformation|GetVelocity)))
    (:then_1
      (Rendering|SetVisibility (Variables|Default|GetCharacterBody) Reverse false))
    (:then_2
      (Variables|/Script/Engine.SpringArmComponent|SetbDoCollisionTest (Variables|Default|GetSpringArm) Reverse)
      (Pawn|Components|CharacterMovement|SetMovementMode (Variables|Character|GetCharacterMovement) (select Reverse "MOVE_Walking" "MOVE_None") 0)
      (Collision|SetCollisionEnabled (Variables|Collision|GetCapsuleComponent) (select Reverse "QueryAndPhysics" "NoCollision")))
    (:then_3
      (return))))